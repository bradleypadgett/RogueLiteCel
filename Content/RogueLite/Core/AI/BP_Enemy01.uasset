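; BP_Enemy01 is a roguelite enemy that moves along its Z axis through a timeline and destroys itself on Died.
; BeginPlay starts the timeline at a random time, and each update applies the track value as a swept local offset.
; The Hit event is empty; the HealthComp damage logic, with doubled headshot damage detected by "Head" in the component name, is disconnected and never runs.
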(event EventBeginPlay
  (Utilities|FlowControl|Sequence
    (:then_0
      (bind _newtrack_1 (Timeline|Timeline_0 SetNewTime)
        (:Update
          (Transformation|AddActorLocalOffset (Math|Vector|MakeVector 0.0 0.0 _newtrack_1) true false))))
    (:then_1
      (Timeline|Timeline_0 Play))))

(event EventDied
  (Actor|DestroyActor))

(event EventHit
  (params (Hit :type Hit%20Result%20Structure) (Damage :type Integer) (Damage%20Multiplier :type Integer)))

(fn ConstructionScript)