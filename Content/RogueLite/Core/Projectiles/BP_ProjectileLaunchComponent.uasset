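; Launcher component that spawns a projectile actor of a configurable class at its own world transform.
; LaunchProjectile sets the spawned actor's ProjectileMovementComponent velocity to a direction times Speed.
; For player shots TargetLocation serves directly as the direction; otherwise it uses the unit vector from TargetLocation toward the component.
; The Collision input is unused, and alternate spawn, warning and emitter nodes are disconnected.
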(event Custom|Launch%20Projectile
  (params (Target%20Location :type Vector) (Collision :type Boolean) (Player :type Boolean))
  (Variables|Internal|SetTarget%20Location Target%20Location)
  (if Player
    _
    (else
      _))
  (bind _returnvalue (Game|SpawnActorfromClass (Variables|Editable|GetClass) (Transformation|GetWorldTransform) "Undefined" 0 0))
  (Utilities|IsValid _returnvalue
    (:Is%20Valid
      (Variables|Internal|SetProjectile%20Movement%20Component%20Ref (Actor|GetComponentbyClass _returnvalue "/Script/Engine.ProjectileMovementComponent"))
      (Utilities|IsValid (Variables|Internal|GetProjectile%20Movement%20Component%20Ref)
        (:Is%20Valid
          (Variables|/Script/Engine.MovementComponent|SetVelocity (Variables|Internal|GetProjectile%20Movement%20Component%20Ref) (* (Math|Vector|SelectVector (Variables|Internal|GetTarget%20Location) (Math|Vector|GetUnitDirection(Vector) (Variables|Internal|GetTarget%20Location) (Transformation|GetWorldLocation)) Player) (Variables|Editable|GetSpeed))))))))