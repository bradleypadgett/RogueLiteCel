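; BP_ImpulseBullet is a delayed magic explosion that damages and shoves patrolling AI around its spawn point.
; On BeginPlay it traces down to place its radial force on the ground, plays a sound, waits ExplosionDelay, then damages overlapping BP_PatrollingAI and halts their movement for a second.
; It fires the impulse with a timeline-driven light flash; the sphere trace result is unused.
; The construction script feeds delay and color to Niagara and the light.
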(event EventBeginPlay
  (bind _defaultsceneroot (Variables|Default|GetDefaultSceneRoot))
  (bind _defaultsceneroot_2 (Variables|Default|GetDefaultSceneRoot))
  (bind _returnvalue (Transformation|GetWorldLocation _defaultsceneroot))
  (bind _returnvalue_2 (Transformation|GetWorldLocation _defaultsceneroot_2))
  (bind (_outhits _returnvalue_3) (Class|KismetSystemLibrary|LineTraceMultiforObjects _returnvalue_2 (- _returnvalue_2 "0.000000, 0,150.000000") (Utilities|Array|MakeArray "ObjectTypeQuery1") true 0 "None" true))
  (if _returnvalue_3
    (for _array_element _outhits
      (Transformation|SetWorldLocation (Variables|Default|GetRadialForce) (.location _array_element) false true)))
  (Audio|PlaySoundatLocation "/Game/RogueLite/Audio/MagicExplosion_Cue.MagicExplosion_Cue" (Transformation|GetActorLocation) "0, 0, 0" 1.0 1.0 0.0 0 0 0)
  (Utilities|FlowControl|Delay (Variables|Default|GetExplosionDelay))
  (Collision|MultiSphereTraceByChannel _returnvalue _returnvalue 2e+03 "TraceTypeQuery1" false 0 "None")
  (bind _output_get (Variables|Default|SetOverlapping%20Actors (Collision|GetOverlappingActors (Variables|Default|GetSphere1) "/Game/RogueLite/Core/AI/Enemies/BP_PatrollingAI.BP_PatrollingAI_C" :!class /Script/Engine.PrimitiveComponent)))
  (for _array_element_2 _output_get
    (Development|PrintString (Utilities|GetDisplayName _array_element_2) true true "(R=0.000000,G=1.000000,B=0.250000,A=1.000000)")
    (bind _asbp_patrolling_ai (Utilities|Casting|CastToBP_PatrollingAI _array_element_2))
    (Default|SetMove _asbp_patrolling_ai false)
    (Class|BPIHit|Hit(Message) :self (Variables|/Game/RogueLite/Core/AI/Enemies/BP_PatrollingAI.BP_PatrollingAI_C|GetHealthComp _asbp_patrolling_ai) :Damage 50 :Damage%20Multiplier 1))
  (Utilities|FlowControl|Sequence
    (:then_0
      (Class|RadialForceComponent|FireImpulse (Variables|Default|GetRadialForce))
      (bind _brightness (Timeline|Brightness Play)
        (:Update
          (Rendering|Components|Light|SetIntensity (Variables|Default|GetPointLight) (* 100 _brightness)))))
    (:then_1
      (Utilities|FlowControl|Delay 1.0)
      (for _array_element_3 (Variables|Default|GetOverlapping%20Actors)
        (bind _asbp_patrolling_ai_2 (Utilities|Casting|CastToBP_PatrollingAI _array_element_3))
        (Default|SetMove _asbp_patrolling_ai_2 true)))))

(event Collision|EventActorBeginOverlap
  (params (OtherActor :type Actor%20Object%20Reference)))

(event EventTick
  (params (DeltaSeconds :type Float%20%28single-precision%29)))

(fn ConstructionScript
  (Effects|Components|ParticleSystem|SetFloatParameter (Variables|Default|GetNiagara) "ExplosionDelay" (Variables|Default|GetExplosionDelay))
  (Effects|Components|ParticleSystem|SetColorParameter (Variables|Default|GetNiagara) "Color" (Variables|Default|GetColor))
  (Rendering|Components|Light|SetLightColor (Variables|Default|GetPointLight) (Variables|Default|GetColor) true))