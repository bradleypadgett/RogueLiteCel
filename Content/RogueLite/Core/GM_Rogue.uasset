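; GM_Rogue is the roguelite's game mode, which sets up the crosshair HUD and player settings on BeginPlay.
; It loads the SG_Save slot if present, applying volume through a sound mix class override and copying sensitivity to BP_RoguePlayer.
; Otherwise it creates and saves default settings, applying only the volume.
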(event EventBeginPlay
  (bind _returnvalue (UserInterface|CreateWidget "/Game/RogueLite/Misc/Crosshair/WBP_Crosshair.WBP_Crosshair_C" (Game|GetPlayerController 0)))
  (UserInterface|Viewport|AddtoViewport _returnvalue 0)
  (bind _returnvalue_2 (SaveGame|DoesSaveGameExist "1"))
  (if _returnvalue_2
    (bind _returnvalue_3 (SaveGame|LoadGamefromSlot "1"))
    (bind _assg_save (Utilities|Casting|CastToSG_Save _returnvalue_3))
    (Audio|SetSoundMixClassOverride "/Game/RogueLite/Audio/SFXMix.SFXMix" "/Engine/EngineSounds/Master.Master" (/ (Math|Conversions|ToFloat(Integer) (Variables|/Game/RogueLite/SaveGame/SG_Save.SG_Save_C|GetVolume _assg_save)) 1e+02) 1.0 1.0 true)
    (Audio|PushSoundMixModifier "/Game/RogueLite/Audio/SFXMix.SFXMix")
    (bind _asbp_rogue_player (Utilities|Casting|CastToBP_RoguePlayer (Game|GetPlayerCharacter 0)))
    (Variables|/Game/RogueLite/Core/Player/BP_RoguePlayer.BP_RoguePlayer_C|SetSens _asbp_rogue_player (Variables|/Game/RogueLite/SaveGame/SG_Save.SG_Save_C|GetSensitivity _assg_save))
    (else
      (bind _returnvalue_4 (SaveGame|CreateSaveGameObject "/Game/RogueLite/SaveGame/SG_Save.SG_Save_C"))
      (Variables|/Game/RogueLite/SaveGame/SG_Save.SG_Save_C|SetVolume _returnvalue_4 50)
      (Variables|/Game/RogueLite/SaveGame/SG_Save.SG_Save_C|SetSensitivity _returnvalue_4 25)
      (SaveGame|SaveGametoSlot _returnvalue_4 "1")
      (Audio|SetSoundMixClassOverride "/Game/RogueLite/Audio/SFXMix.SFXMix" "/Engine/EngineSounds/Master.Master" (/ (Math|Conversions|ToFloat(Integer) (Variables|/Game/RogueLite/SaveGame/SG_Save.SG_Save_C|GetVolume _returnvalue_4)) 1e+02) 1.0 1.0 true)
      (Audio|PushSoundMixModifier "/Game/RogueLite/Audio/SFXMix.SFXMix"))))

(fn ConstructionScript)