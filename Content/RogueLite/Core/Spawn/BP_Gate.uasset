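; BP_Gate is a level-exit portal that starts with collision off and its material faded out.
; Open waits through a delay, then OpenPortal unhides the cube and a timeline fades in the Fresnel parameter on a dynamic MI_Portal material.
; Collision turns on only when the fade finishes, after which the player character overlapping the cube loads TestLevel.
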(event OnComponentBeginOverlap(Cube)
  (params (OverlappedComponent :type Primitive%20Component%20Object%20Reference) (OtherActor :type Actor%20Object%20Reference) (OtherComp :type Primitive%20Component%20Object%20Reference) (OtherBodyIndex :type Integer) (bFromSweep :type Boolean) (SweepResult :type Hit%20Result%20Structure%20%28by%20ref%29))
  (if (== OtherActor (Game|GetPlayerCharacter 0))
    (Game|OpenLevel(byName) "TestLevel")))

(event Custom|Open%20Portal
  (Development|SetHiddeninGame (Variables|Default|GetCube) false false)
  (bind _newtrack_0 (Timeline|Open%20Portal%20Timeline PlayFromStart)
    (:Update
      (Rendering|Material|SetScalarParameterValue (Variables|Default|GetMI) "Fresnel" (Math|Float|Lerp -2.0 0.5 _newtrack_0) :!class /Script/Engine.MaterialInstanceDynamic))
    (:Finished
      (Collision|SetCollisionEnabled (Variables|Default|GetCube) "QueryAndPhysics"))))

(event Custom|Open
  (Utilities|FlowControl|Delay 1e+01)
  (CallFunction|OpenPortal))

(event EventBeginPlay
  (bind _returnvalue (Rendering|Material|CreateDynamicMaterialInstance (Variables|Default|GetCube) 0 "/Game/RogueLite/VFX/Portal/MI_Portal.MI_Portal" "None" :!class /Script/Engine.PrimitiveComponent))
  (Variables|Default|SetMI _returnvalue)
  (Rendering|Material|SetScalarParameterValue (Variables|Default|GetMI) "Fresnel" -2.0 :!class /Script/Engine.MaterialInstanceDynamic)
  (Collision|SetCollisionEnabled (Variables|Default|GetCube) "NoCollision"))

(fn ConstructionScript)