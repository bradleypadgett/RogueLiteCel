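; BP_SpawnLocations is a spawn point marker actor typed as Empty, Chest, Orb or Gate through its SpawnType setting.
; Its construction script uses that type to pick the billboard sprite and scale, making each kind visually distinct.
; The same script replaces the actor's tags with one matching the type name, or "None" for Empty.
; It has no runtime logic, as BeginPlay is empty.
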(event EventBeginPlay)

(fn ConstructionScript
  (bind _spawn_type (Variables|Spawn|GetSpawn%20Type))
  (bind _returnvalue (Utilities|Select :Index _spawn_type :NewEnumerator0 1e+01 :NewEnumerator1 1.0 :NewEnumerator2 1.0 :NewEnumerator3 3.0))
  (Variables|/Script/Engine.BillboardComponent|SetSprite (Variables|Default|GetBillboard1) (Utilities|Select :Index (Variables|Spawn|GetSpawn%20Type) :NewEnumerator0 "/Engine/EditorMaterials/MatineeGroups/MAT_Groups_Float.MAT_Groups_Float" :NewEnumerator1 "/Engine/EditorResources/Spawn_Point.Spawn_Point" :NewEnumerator2 "/Engine/EditorResources/S_PortalActorIcon.S_PortalActorIcon" :NewEnumerator3 "/Engine/EngineResources/AICON-Green.AICON-Green"))
  (Transformation|SetWorldScale3D (Variables|Default|GetBillboard1) (Math|Vector|MakeVector _returnvalue _returnvalue _returnvalue))
  (Variables|Default|SetTags (Utilities|Array|MakeArray (Utilities|Select :Index (Variables|Spawn|GetSpawn%20Type) :NewEnumerator0 "None" :NewEnumerator1 "Chest" :NewEnumerator2 "Orb" :NewEnumerator3 "Gate"))))