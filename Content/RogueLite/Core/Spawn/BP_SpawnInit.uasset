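; BP_SpawnInit randomly populates the roguelite level with chests, orbs and a gate when play begins.
; Each spawner gathers BP_SpawnLocations actors by tag, then picks points at random without repeats up to a configurable count.
; Chests get slight random sink and tilt, gates a random yaw, and orbs are raised, scaled down and colored by spawn order.
; Only the chest loop guards against running out of locations.
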(event Custom|Spawn%20Chests
  (bind _outactors (Actor|GetAllActorsOfClasswithTag "/Game/RogueLite/Core/Spawn/BP_SpawnLocations.BP_SpawnLocations_C" "Chest"))
  (Variables|Default|SetChest%20Locations _outactors)
  (Utilities|FlowControl|ForLoopwithBreak 1 (Variables|Spawns|GetChest%20Spawns) :!label _label
    (:LoopBody
      (if (> (Utilities|Array|Length (Variables|Default|GetChest%20Locations)) 0)
        (bind _output_get (Variables|Default|SetTemp%20Chest (.OutItem (Utilities|Array|Random (Variables|Default|GetChest%20Locations)))))
        (Utilities|Array|RemoveItem (Variables|Default|GetChest%20Locations) _output_get)
        (Game|SpawnActorfromClass "/Game/RogueLite/Core/Items/BP_Chest.BP_Chest_C" (Math|Transform|MakeTransform (Math|Vector|MakeVector (.X (Math|Vector|BreakVector (Transformation|GetActorLocation (Variables|Default|GetTemp%20Chest)))) (.Y (Math|Vector|BreakVector (Transformation|GetActorLocation (Variables|Default|GetTemp%20Chest)))) (- (.Z (Math|Vector|BreakVector (Transformation|GetActorLocation (Variables|Default|GetTemp%20Chest)))) (Math|Random|RandomFloatinRange 0.0 5.0))) (Math|Rotator|MakeRotator (Math|Random|RandomFloatinRange -1e+01 0.0) (Math|Random|RandomFloatinRange -5.0 5.0) (Math|Random|RandomFloatinRange 0.0 3.6e+02)) "1,1,1") "Undefined" 0 0)
        (else
          (goto _label Break))))))

(event Custom|Spawn%20Orbs
  (bind _outactors (Actor|GetAllActorsOfClasswithTag "/Game/RogueLite/Core/Spawn/BP_SpawnLocations.BP_SpawnLocations_C" "Orb"))
  (Variables|Default|SetOrb%20Locations _outactors)
  (bind _index (Utilities|FlowControl|ForLoopwithBreak 1 (Variables|Spawns|GetOrb%20Spawns))
    (:LoopBody
      (Variables|Default|SetOrb%20Index _index)
      (bind _output_get (Variables|Default|SetTemp%20Orb (.OutItem (Utilities|Array|Random (Variables|Default|GetOrb%20Locations)))))
      (Utilities|Array|RemoveItem (Variables|Default|GetOrb%20Locations) _output_get)
      (bind _returnvalue (Game|SpawnActorfromClass "/Game/RogueLite/Core/Items/BP_Orb1.BP_Orb1_C" (Math|Transform|MakeTransform (Math|Vector|MakeVector (.x (Transformation|GetActorLocation (Variables|Default|GetTemp%20Orb))) (.y (Transformation|GetActorLocation (Variables|Default|GetTemp%20Orb))) (+ (.z (Transformation|GetActorLocation (Variables|Default|GetTemp%20Orb))) 1e+02)) "0, 0, 0" "1,1,1") "Undefined" 0 0))
      (Default|SetScale _returnvalue 0.25)
      (Default|SetColor _returnvalue (Utilities|Select :Index (- (Variables|Default|GetOrb%20Index) 1) :Option%200 "(R=0.000000,G=0.333333,B=1.000000,A=1.000000)" :Option%201 "(R=1.000000,G=0.023286,B=0.000000,A=1.000000)" :Option%202 "(R=0.000000,G=1.000000,B=0.125580,A=1.000000)")))))

(event Custom|Spawn%20Gate
  (bind _outactors (Actor|GetAllActorsOfClasswithTag "/Game/RogueLite/Core/Spawn/BP_SpawnLocations.BP_SpawnLocations_C" "Gate"))
  (Variables|Default|SetGate%20Location _outactors)
  (Utilities|FlowControl|ForLoopwithBreak 1 (Variables|Spawns|GetGate%20Spawns)
    (:LoopBody
      (bind _output_get (Variables|Default|SetTemp%20Gate (.OutItem (Utilities|Array|Random (Variables|Default|GetGate%20Location)))))
      (Utilities|Array|RemoveItem (Variables|Default|GetGate%20Location) _output_get)
      (Game|SpawnActorfromClass "/Game/RogueLite/Core/Spawn/BP_Gate.BP_Gate_C" (Math|Transform|MakeTransform (Transformation|GetActorLocation (Variables|Default|GetTemp%20Gate)) (Math|Rotator|MakeRotator 0.0 0.0 (Math|Random|RandomFloatinRange 0.0 3.6e+02)) "1,1,1") "Undefined" 0 0))))

(event EventBeginPlay
  (CallFunction|SpawnChests)
  (CallFunction|SpawnOrbs)
  (CallFunction|SpawnGate))

(fn ConstructionScript)