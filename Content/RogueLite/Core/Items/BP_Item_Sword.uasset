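; Sword pickup item for the roguelite that raises the player's base damage when interacted with.
; Interact runs the parent logic, adds a widget labeled "Katana" and adds a flat bonus to the player's BaseDamage.
; BeginPlay, SpawnItem and the construction script only defer to the parent item class.
; Disconnected offset and dash-increment nodes remain in the event graph and never execute.
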(event EventBeginPlay
  (|CallParentFunction))

(event EventSpawnItem
  (|CallParentFunction))

(event EventInteract
  (bind _player (Variables|Default|GetPlayer))
  (|CallParentFunction)
  (CallFunction|AddWidget "Katana")
  (Variables|/Game/RogueLite/Core/Player/BP_RoguePlayer.BP_RoguePlayer_C|SetBase%20Damage _player (+ (Variables|/Game/RogueLite/Core/Player/BP_RoguePlayer.BP_RoguePlayer_C|GetBase%20Damage _player) 5)))

(fn ConstructionScript
  (|CallParentFunction))