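; Roguelite loot chest that opens once on Interact and, after a short delay, spawns a shoes, fan or sword item at random.
; The item appears above a random reachable point nearby, with sounds and a Niagara effect.
; A separately spawned key-cost label shows on sphere overlap while closed; no cost is checked here.
; Render briefly highlights the closed chest via custom depth stencil, held by a retriggerable delay.
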(event OnComponentBeginOverlap(Sphere1)
  (params (OverlappedComponent :type Primitive%20Component%20Object%20Reference) (OtherActor :type Actor%20Object%20Reference) (OtherComp :type Primitive%20Component%20Object%20Reference) (OtherBodyIndex :type Integer) (bFromSweep :type Boolean) (SweepResult :type Hit%20Result%20Structure%20%28by%20ref%29))
  (if (not (Variables|Default|GetOpen))
    (Rendering|SetVisibility (Variables|Default|GetText%20Render) true false)))

(event OnComponentEndOverlap(Sphere1)
  (params (OverlappedComponent :type Primitive%20Component%20Object%20Reference) (OtherActor :type Actor%20Object%20Reference) (OtherComp :type Primitive%20Component%20Object%20Reference) (OtherBodyIndex :type Integer))
  (Rendering|SetVisibility (Variables|Default|GetText%20Render) false false))

(event Custom|Interact
  (bind _returnvalue (Transformation|GetActorLocation))
  (bind _ns_openchest (Variables|Default|GetNS_OpenChest))
  (if (not (Variables|Default|GetOpen))
    (Rendering|SetRenderCustomDepth (Variables|Default|GetSkeletalMesh) true)
    (Variables|Default|SetOpen true)
    (Rendering|SetVisibility (Variables|Default|GetText%20Render) false false)
    (Audio|PlaySoundatLocation "/Game/RogueLite/Audio/OpenChest.OpenChest" (Transformation|GetActorLocation) "0, 0, 0" 1.0 1.0 0.0 0 0 0)
    (Utilities|FlowControl|Delay 1.5)
    (Audio|PlaySoundatLocation "/Game/RogueLite/Audio/PopCue.PopCue" _returnvalue "0, 0, 0" 1.0 1.0 0.0 0 0 0)
    (bind _output_get (Variables|Default|SetSpawn%20Location (+ (.RandomLocation (AI|Navigation|GetRandomReachablePointinRadius _returnvalue 1.5e+02 0 0)) "0, 0,100.000000")))
    (Game|SpawnActorfromClass (Utilities|Select :Index (Math|Random|RandomIntegerinRange 0 2) :Option%200 "/Game/RogueLite/Core/Items/BP_Item_Shoes.BP_Item_Shoes_C" :Option%201 "/Game/RogueLite/Core/Items/BP_Item_Fan.BP_Item_Fan_C" :Option%202 "/Game/RogueLite/Core/Items/BP_Item_Sword.BP_Item_Sword_C") (Math|Transform|MakeTransform _output_get "0, 0, 0" "1,1,1") "Undefined" 0 0)
    (Transformation|SetWorldLocation _ns_openchest (Variables|Default|GetSpawn%20Location) false true)
    (Class|NiagaraComponent|SetAsset _ns_openchest "/Game/RogueLite/VFX/ChestOpen/NS_OpenChest.NS_OpenChest")))

(event Custom|Render
  (bind _skeletalmesh (Variables|Default|GetSkeletalMesh))
  (if (not (Variables|Default|GetOpen))
    (Rendering|SetRenderCustomDepth _skeletalmesh true)
    (Rendering|SetCustomDepthStencilValue _skeletalmesh 1)
    (Utilities|FlowControl|RetriggerableDelay 0.1)
    (Rendering|SetRenderCustomDepth _skeletalmesh false)
    (Rendering|SetCustomDepthStencilValue _skeletalmesh 0)))

(event EventBeginPlay
  (bind _returnvalue (Transformation|GetActorTransform))
  (bind _returnvalue_2 (Math|Random|RandomIntegerinRange 5 10))
  (bind _returnvalue_3 (* _returnvalue_2 4 1))
  (bind _returnvalue_4 (Math|Conversions|ToFloat(Integer) _returnvalue_3))
  (Variables|Default|SetCost 1)
  (bind _returnvalue_5 (Game|SpawnActorfromClass "/Game/RogueLite/Core/Health/BP_CostText.BP_CostText_C" (Math|Transform|MakeTransform (Math|Vector|MakeVector (+ (.x (.location _returnvalue)) _returnvalue_4) (+ (.y (.location _returnvalue)) _returnvalue_4) (+ (.z (.location _returnvalue)) _returnvalue_4)) "0, 0, 0" "1,1,1") "Undefined" 0 0))
  (Rendering|Components|TextRender|SetText (Variables|/Game/RogueLite/Core/Health/BP_CostText.BP_CostText_C|GetTextRender _returnvalue_5) (Utilities|Text|ToText(String) (Utilities|String|Append (Utilities|String|ToString(Integer) (Variables|Default|GetCost)) " Key")))
  (bind _output_get (Variables|Default|SetText%20Render (Variables|/Game/RogueLite/Core/Health/BP_CostText.BP_CostText_C|GetTextRender _returnvalue_5)))
  (Rendering|SetVisibility _output_get false false))

(fn ConstructionScript)