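; BP_Item_Helmet is a roguelite item that raises the player's maximum health by a fixed amount on interaction.
; It extends a parent item class, passing BeginPlay, SpawnItem and construction straight through.
; Interact runs the parent logic, adds a "Helmet" widget, increases HealthComp's MaxHealth, refreshes the health visual and calls HealthTimer.
; An unconnected node that would also add to current health never runs.
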(event EventBeginPlay
  (|CallParentFunction))

(event EventSpawnItem
  (|CallParentFunction))

(event EventInteract
  (bind _player (Variables|Default|GetPlayer))
  (bind _healthcomp (Variables|/Game/RogueLite/Core/Player/BP_RoguePlayer.BP_RoguePlayer_C|GetHealthComp _player))
  (|CallParentFunction)
  (CallFunction|AddWidget "Helmet")
  (Variables|/Game/RogueLite/Core/Health/BP_HealthComponent.BP_HealthComponent_C|SetMax%20Health _healthcomp (+ (Variables|/Game/RogueLite/Core/Health/BP_HealthComponent.BP_HealthComponent_C|GetMax%20Health _healthcomp) 25.0))
  (Default|UpdateHealthVisual _healthcomp true)
  (Default|HealthTimer _healthcomp))

(fn ConstructionScript
  (|CallParentFunction))