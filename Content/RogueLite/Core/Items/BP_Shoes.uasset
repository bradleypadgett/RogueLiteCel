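; BP_Shoes is a roguelite item that permanently raises the player's movement speed when interacted with.
; It inherits spawn and interaction logic from its parent, then adds a flat bonus to the player's CharacterMovement MaxWalkSpeed on Interact.
; A disconnected branch that would also grant an extra dash charge remains in the graph but never runs.
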(event EventBeginPlay
  (|CallParentFunction))

(event EventSpawnItem
  (|CallParentFunction))

(event EventInteract
  (bind _player (Variables|Default|GetPlayer))
  (bind _charactermovement (Variables|/Script/Engine.Character|GetCharacterMovement _player))
  (|CallParentFunction)
  (Variables|/Script/Engine.CharacterMovementComponent|SetMaxWalkSpeed _charactermovement (+ (Variables|/Script/Engine.CharacterMovementComponent|GetMaxWalkSpeed _charactermovement) 4e+01)))

(fn ConstructionScript
  (|CallParentFunction))