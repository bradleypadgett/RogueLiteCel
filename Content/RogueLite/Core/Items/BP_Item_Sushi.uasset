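; BP_Item_Sushi is a roguelite item that restores health to the player when interacted with.
; Interact runs the parent item logic, adds a "Sushi" widget, and raises the player's HealthComp amount by a flat value, clamped between zero and its Health value.
; It then refreshes the health visual and calls HealthTimer on that component.
; BeginPlay and SpawnItem only forward to the parent class.
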(event EventBeginPlay
  (|CallParentFunction))

(event EventSpawnItem
  (|CallParentFunction))

(event EventInteract
  (bind _player (Variables|Default|GetPlayer))
  (bind _healthcomp (Variables|/Game/RogueLite/Core/Player/BP_RoguePlayer.BP_RoguePlayer_C|GetHealthComp _player))
  (|CallParentFunction)
  (CallFunction|AddWidget "Sushi")
  (Variables|/Game/RogueLite/Core/Health/BP_HealthComponent.BP_HealthComponent_C|SetHealth%20Amount _healthcomp (Math|Float|Clamp(Float) (+ (Variables|/Game/RogueLite/Core/Health/BP_HealthComponent.BP_HealthComponent_C|GetHealth%20Amount _healthcomp) 25.0) 0.0 (Math|Conversions|ToFloat(Integer) (Variables|/Game/RogueLite/Core/Health/BP_HealthComponent.BP_HealthComponent_C|GetHealth _healthcomp))))
  (Default|UpdateHealthVisual _healthcomp true)
  (Default|HealthTimer _healthcomp))

(fn ConstructionScript
  (|CallParentFunction))