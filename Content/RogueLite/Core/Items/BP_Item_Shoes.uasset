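; BP_Item_Shoes is a roguelite item that grants the player an extra dash on interaction.
; It defers spawn, setup and base interaction to its parent item class, then adds a "Shoes" widget and increments both maximum and current dashes.
; A walk speed increase is also present in the graph but is disconnected and never runs.
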(event EventBeginPlay
  (|CallParentFunction))

(event EventSpawnItem
  (|CallParentFunction))

(event EventInteract
  (bind _player (Variables|Default|GetPlayer))
  (|CallParentFunction)
  (CallFunction|AddWidget "Shoes")
  (Math|Integer|IncrementInt (Variables|/Game/RogueLite/Core/Player/BP_RoguePlayer.BP_RoguePlayer_C|GetMaxDashes _player)
    (:%20%20
      (Math|Integer|IncrementInt (Variables|/Game/RogueLite/Core/Player/BP_RoguePlayer.BP_RoguePlayer_C|GetDashes _player)))))

(fn ConstructionScript
  (|CallParentFunction))