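; BP_Item is a roguelite pickup actor that bobs in place and is consumed when the player touches it.
; On BeginPlay it caches the BP_RoguePlayer pawn, activates its Niagara effect and starts a randomized timeline that nudges the mesh along Z.
; A sphere overlap with that player calls Interact, which only prints a debug string and destroys the item.
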(event OnComponentBeginOverlap(Sphere)
  (params (OverlappedComponent :type Primitive%20Component%20Object%20Reference) (OtherActor :type Actor%20Object%20Reference) (OtherComp :type Primitive%20Component%20Object%20Reference) (OtherBodyIndex :type Integer) (bFromSweep :type Boolean) (SweepResult :type Hit%20Result%20Structure%20%28by%20ref%29))
  (if (== OtherActor (Variables|Default|GetPlayer))
    (CallFunction|Interact)))

(event Custom|Interact
  (Development|PrintString "Interact" true true "(R=1.000000,G=0.000000,B=0.734174,A=1.000000)")
  (Actor|DestroyActor))

(event Custom|Spawn%20Item
  (Components|Activation|Activate (Variables|Default|GetNiagara) false))

(event EventBeginPlay
  (bind _asbp_rogue_player (Utilities|Casting|CastToBP_RoguePlayer (Game|Player|GetPlayerPawn 0)))
  (Variables|Default|SetPlayer _asbp_rogue_player)
  (CallFunction|SpawnItem)
  (Utilities|FlowControl|Sequence
    (:then_0
      (bind _newtrack_0 (Timeline|Location%20Offset Play)
        (:Update
          (Transformation|AddLocalOffset (Variables|Default|GetStaticMesh) (Math|Vector|MakeVector 0.0 0.0 (/ _newtrack_0 5.0)) false true))))
    (:then_1
      (Timeline|Location%20Offset SetNewTime))))

(fn ConstructionScript)