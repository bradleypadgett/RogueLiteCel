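; Health component that tracks its owner's health, handles damage and healing, and sends a died message when damage is lethal.
; Hit doubles damage on components named "Head" and applies a multiplier, while LoseHealth applies raw damage.
; Damage spawns randomly offset damage text and updates a material billboard bar's fill and color.
; A retriggerable timer hides the bar after inactivity unless KeepHealthOnScreen is set.
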(event Custom|LoseHealth
  (params (Damage :type Integer) (bHeadshot :type Boolean))
  (bind _returnvalue (Components|GetOwner))
  (bind _returnvalue_2 (Math|Random|RandomIntegerinRange 5 10))
  (bind _returnvalue_3 (Math|Random|RandomBool))
  (bind _returnvalue_4 (Transformation|GetActorTransform _returnvalue))
  (bind _returnvalue_5 (Math|Integer|SelectInt 1 -1 _returnvalue_3))
  (bind _returnvalue_6 (* _returnvalue_2 5 _returnvalue_5))
  (bind _returnvalue_7 (Math|Conversions|ToFloat(Integer) _returnvalue_6))
  (Variables|Default|SetDamage Damage)
  (CallFunction|HealthTimer)
  (if (> (- (Variables|Default|GetHealth%20Amount) (Math|Conversions|ToFloat(Integer) (Variables|Default|GetDamage))) 0.0)
    (Variables|Default|SetHealth%20Amount (- (Variables|Default|GetHealth%20Amount) (Math|Conversions|ToFloat(Integer) (Variables|Default|GetDamage))))
    (CallFunction|UpdateHealthVisual true :!label _label)
    (bind _returnvalue_8 (Game|SpawnActorfromClass "/Game/RogueLite/Core/Health/BP_DamageText.BP_DamageText_C" (Math|Transform|MakeTransform (Math|Vector|MakeVector (+ (.x (.location _returnvalue_4)) _returnvalue_7) (+ (.y (.location _returnvalue_4)) _returnvalue_7) (+ (.z (.location _returnvalue_4)) _returnvalue_7)) "0, 0, 0" "1,1,1") "Undefined" 0 0))
    (Rendering|Components|TextRender|SetText (Variables|/Game/RogueLite/Core/Health/BP_DamageText.BP_DamageText_C|GetTextRender _returnvalue_8) (Utilities|Text|ToText(Integer) (Variables|Default|GetDamage)))
    (Rendering|Components|TextRender|SetTextRenderColor (Variables|/Game/RogueLite/Core/Health/BP_DamageText.BP_DamageText_C|GetTextRender _returnvalue_8) (Math|Conversions|ToColor(LinearColor) (Math|Color|SelectColor "(R=0.916667,G=0.037713,B=0.028595,A=1.000000)" "(R=0.968750,G=0.400023,B=0.033262,A=1.000000)" false) false))
    (else
      (Utilities|FlowControl|Sequence
        (:then_0
          (goto _label))
        (:then_1
          (Class|BPIHit|Died(Message) (Components|GetOwner)))))))

(event Custom|Health%20Timer
  (Utilities|FlowControl|RetriggerableDelay 1e+01)
  (if (not (Variables|Default|GetbKeepHealthOnScreen))
    (Rendering|Material|SetScalarParameterValue (Variables|Default|GetHealth%20Decal) "Health" 0.0 :!class /Script/Engine.MaterialInstanceDynamic)))

(event Custom|Initialize%20Health
  (bind _output_get (Variables|Default|SetMax%20Health (Math|Conversions|ToFloat(Integer) (Variables|Default|GetHealth))))
  (Variables|Default|SetHealth%20Amount _output_get))

(event Custom|Update%20Health%20Visual
  (params (bVisible :type Boolean))
  (bind _health_decal (Variables|Default|GetHealth%20Decal))
  (Rendering|Material|SetScalarParameterValue _health_decal "Health" (Math|Float|SelectFloat (/ (Variables|Default|GetHealth%20Amount) (Variables|Default|GetMax%20Health)) 0.0 bVisible) :!class /Script/Engine.MaterialInstanceDynamic)
  (Rendering|Material|SetVectorParameterValue _health_decal "Color" (Utilities|Select :Index (Math|Float|Truncate (* 3 (/ (Variables|Default|GetHealth%20Amount) (Variables|Default|GetMax%20Health)))) :Option%200 "(R=0.725490,G=0.031373,B=0.050980,A=1.000000)" :Option%201 "(R=0.725490,G=0.702353,B=0.031373,A=1.000000)" :Option%202 "(R=0.030713,G=0.730461,B=0.205079,A=1.000000)" :Option%203 "(R=0.030713,G=0.730461,B=0.205079,A=1.000000)") :!class /Script/Engine.MaterialInstanceDynamic))

(event Custom|GainHealth
  (params (Health%20Gain :type Integer))
  (Variables|Default|SetHealth%20Amount (Math|Float|Clamp(Float) (+ (Variables|Default|GetHealth%20Amount) (Math|Conversions|ToFloat(Integer) Health%20Gain)) 0.0 (Variables|Default|GetMax%20Health))))

(event EventBeginPlay
  (CallFunction|InitializeHealth)
  (bind _returnvalue (Game|AddComponentbyClass (Components|GetOwner) (Variables|Default|GetHealth%20Billboard%20Class) false (Math|Transform|MakeTransform (Math|Vector|MakeVector 0.0 0.0 (Math|Conversions|ToFloat(Integer) (Variables|Default|GetRelative%20Transform%20Location%20Z))) "0, 0, 0" "1,1,1")))
  (bind _output_get (Variables|Default|SetHealth%20Billboard _returnvalue))
  (Class|MaterialBillboardComponent|SetElements _output_get (Utilities|Array|MakeArray (Utilities|Struct|MakeMaterialSpriteElement "/Game/RogueLite/Core/Health/MI_Health.MI_Health" 0 false 5.0 5e+01)))
  (bind _returnvalue_2 (Rendering|Material|CreateDynamicMaterialInstance _output_get 0 "/Game/RogueLite/Core/Health/MI_Health.MI_Health" "HealthDecal" :!class /Script/Engine.PrimitiveComponent))
  (Variables|Default|SetHealth%20Decal _returnvalue_2))

(event EventHit
  (params (Hit :type Hit%20Result%20Structure) (Damage :type Integer) (Damage%20Multiplier :type Integer))
  (bind _returnvalue (Components|GetOwner))
  (bind _returnvalue_2 (Math|Random|RandomIntegerinRange 5 10))
  (bind _returnvalue_3 (Math|Random|RandomBool))
  (bind _returnvalue_4 (Transformation|GetActorTransform _returnvalue))
  (bind _returnvalue_5 (Math|Integer|SelectInt 1 -1 _returnvalue_3))
  (bind _returnvalue_6 (* _returnvalue_2 5 _returnvalue_5))
  (bind _returnvalue_7 (Math|Conversions|ToFloat(Integer) _returnvalue_6))
  (Variables|Default|SetDamage (Math|Float|Truncate (* (Math|Conversions|ToFloat(Integer) Damage) (Math|Conversions|ToFloat(Integer) Damage%20Multiplier) (Math|Float|SelectFloat 2.0 1.0 (Utilities|String|Contains (Utilities|GetDisplayName (.HitComponent (Collision|BreakHitResult Hit))) "Head" true)))))
  (CallFunction|HealthTimer)
  (if (> (- (Variables|Default|GetHealth%20Amount) (Math|Conversions|ToFloat(Integer) (Variables|Default|GetDamage))) 0.0)
    (Variables|Default|SetHealth%20Amount (- (Variables|Default|GetHealth%20Amount) (Math|Conversions|ToFloat(Integer) (Variables|Default|GetDamage))))
    (CallFunction|UpdateHealthVisual true :!label _label)
    (bind _returnvalue_8 (Game|SpawnActorfromClass "/Game/RogueLite/Core/Health/BP_DamageText.BP_DamageText_C" (Math|Transform|MakeTransform (Math|Vector|MakeVector (+ (.x (.location _returnvalue_4)) _returnvalue_7) (+ (.y (.location _returnvalue_4)) _returnvalue_7) (+ (.z (.location _returnvalue_4)) _returnvalue_7)) "0, 0, 0" "1,1,1") "Undefined" 0 0))
    (Rendering|Components|TextRender|SetText (Variables|/Game/RogueLite/Core/Health/BP_DamageText.BP_DamageText_C|GetTextRender _returnvalue_8) (Utilities|Text|ToText(Integer) (Variables|Default|GetDamage)))
    (Rendering|Components|TextRender|SetTextRenderColor (Variables|/Game/RogueLite/Core/Health/BP_DamageText.BP_DamageText_C|GetTextRender _returnvalue_8) (Math|Conversions|ToColor(LinearColor) (Math|Color|SelectColor "(R=0.916667,G=0.037713,B=0.028595,A=1.000000)" "(R=0.968750,G=0.400023,B=0.033262,A=1.000000)" false) false))
    (else
      (Utilities|FlowControl|Sequence
        (:then_0
          (goto _label))
        (:then_1
          (Class|BPIHit|Died(Message) (Components|GetOwner)))))))