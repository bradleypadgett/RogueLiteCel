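; BP_Orb is a visual effects orb actor built from Niagara particles, a point light, layered swirl meshes and an inverted sphere shell.
; The construction script applies Scale, Color and Brightness to these parts, creating dynamic materials for the swirls and a darkened, same-hue back shell.
; On BeginPlay, the SizeThrob timeline animates only the root's world scale as a small offset from the initial Scale.
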(event EventBeginPlay
  (Variables|Default|SetInitScale (Variables|Default|GetScale))
  (bind _update_size (Timeline|Size%20Throb Play)
    (:Update
      (Variables|Default|SetScale (+ (/ _update_size 32.0) (Variables|Default|GetInitScale)))
      (Transformation|SetWorldScale3D (Variables|Default|GetDefaultSceneRoot) (Math|Conversions|ToVector(Float) (Variables|Default|GetScale))))))

(event Collision|EventActorBeginOverlap
  (params (OtherActor :type Actor%20Object%20Reference)))

(event EventTick
  (params (DeltaSeconds :type Float%20%28single-precision%29)))

(fn ConstructionScript
  (bind _color (Variables|Default|GetColor))
  (bind (_h _s) (Math|Color|RGBtoHSV(LinearColor) _color))
  (Transformation|SetWorldScale3D (Variables|Default|GetDefaultSceneRoot) (Math|Conversions|ToVector(Float) (Variables|Default|GetScale)))
  (Niagara|SetNiagaraVariable(Float) (Variables|Default|GetNiagara) "Scale" (Variables|Default|GetScale))
  (Niagara|SetNiagaraVariable(LinearColor) (Variables|Default|GetNiagara) "Color" (Variables|Default|GetColor))
  (Rendering|Components|Light|SetIntensity (Variables|Default|GetPointLight) (Variables|Default|GetBrightness))
  (Rendering|Components|Light|SetLightColor (Variables|Default|GetPointLight) (Variables|Default|GetColor) true)
  (bind _returnvalue (Rendering|Material|CreateDynamicMaterialInstance "/Game/RogueLite/VFX/SphereOrb/MI_OrbSwirls.MI_OrbSwirls" "None" "None" :!class /Script/Engine.KismetMaterialLibrary))
  (Variables|Default|SetMID _returnvalue)
  (Rendering|Material|SetMaterial (Variables|Default|GetSwirls_OuterLayer1) 0 (Variables|Default|GetMID))
  (Rendering|Material|SetVectorParameterValue (Variables|Default|GetMID) "Color" (Variables|Default|GetColor) :!class /Script/Engine.MaterialInstanceDynamic)
  (Rendering|Material|SetScalarParameterValue (Variables|Default|GetMID) "Scale" (Variables|Default|GetScale) :!class /Script/Engine.MaterialInstanceDynamic)
  (bind _returnvalue_2 (Rendering|Material|CreateDynamicMaterialInstance "/Game/RogueLite/VFX/SphereOrb/M_OrbShellBack.M_OrbShellBack" "None" "None" :!class /Script/Engine.KismetMaterialLibrary))
  (Variables|Default|SetMID2 _returnvalue_2)
  (Rendering|Material|SetMaterial (Variables|Default|GetInvertedSphereHQ) 0 (Variables|Default|GetMID2))
  (Rendering|Material|SetVectorParameterValue (Variables|Default|GetMID2) "Color" (Class|KismetMathLibrary|HSVtoRGB _h _s 0.1 1.0) :!class /Script/Engine.MaterialInstanceDynamic))